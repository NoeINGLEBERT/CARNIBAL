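; Game mode for the Game1 level that spawns BP_PlayerManager pawns for connected players.
; It tracks controllers on join and logout, then spawns and possesses pawns for those without one when its spawn events are called.
; ThisAintGonnaWork picks player starts by controller index and starts the HUD.
; Respawn picks a random numbered start, calls the pawn's Respawn and refreshes the HUD through PC_Game1's HUDServer.
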(event `Respawn`
  (for _array_element (`self.PlayerControllers`)
    (if (== (`Controller.K2_GetPawn` _array_element) null)
      (bind _returnvalue (`|SpawnActorFromClass` "/Game/Game/Blueprint/BP_PlayerManager.BP_PlayerManager_C" (`self.GetTransform` (`self.K2_FindPlayerStart` _array_element (`KismetStringLibrary.Conv_IntToString` (`KismetMathLibrary.RandomInteger` 5)))) "Undefined" "MultiplyWithRoot" null null))
      (`Controller.Possess` _array_element _returnvalue)
      (`/Game/Game/Blueprint/BP_PlayerManager.Respawn` _returnvalue)
      (bind _aspc_game_1 (cast `/Game/Game/Levels/Game1/PC_Game1` _array_element)
        (:`then`
          (`/Game/Game/Levels/Game1/PC_Game1.HUD server` _aspc_game_1))
        (:`CastFailed`
          (`KismetSystemLibrary.PrintString` "Ah... bah RIP"))))))

(event `self.K2_OnLogout`
  (params (ExitingController :type "Controller Object Reference"))
  (bind _asplayer_controller (cast `PlayerController` ExitingController))
  (`KismetArrayLibrary.Array_RemoveItem` (`self.PlayerControllers`) _asplayer_controller))

(event `ThisAintGonnaWork`
  (for (_array_element _array_index) (`self.PlayerControllers`)
    (if (== (`Controller.K2_GetPawn` _array_element) null)
      (bind _returnvalue (`|SpawnActorFromClass` "/Game/Game/Blueprint/BP_PlayerManager.BP_PlayerManager_C" (`self.GetTransform` (`self.K2_FindPlayerStart` _array_element (`KismetStringLibrary.Conv_IntToString` _array_index))) "Undefined" "MultiplyWithRoot" null null))
      (`Controller.Possess` _array_element _returnvalue)
      (bind _aspc_game_1 (cast `/Game/Game/Levels/Game1/PC_Game1` _array_element))
      (`/Game/Game/Levels/Game1/PC_Game1.StartHUD` _aspc_game_1))))

(event `self.HandleStartingNewPlayer`
  (params (NewPlayer :type "PlayerController Object Reference"))
  (`KismetArrayLibrary.Array_AddUnique` (`self.PlayerControllers`) NewPlayer))

(fn `DefeatClient`)

(fn `UserConstructionScript`)