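; PC_Game1 is the player controller for Game1, handling the in-game HUD, the death screen and a timed defeat.
; StartHUD chains through HUDserver to HUDclient, which rebuilds WBP_HUD on the local controller, fades it in and hands it to the possessed BP_PlayerManager.
; The same event starts a ten-minute timer to DefeatServer, which spawns BP_Endgame and triggers defeat.
; DeathHUDServer shows WBP_Death for the local controller.
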(event `HUD server`
  (`self.HUD client`))

(event `DefeatServer`
  (bind _returnvalue (`|SpawnActorFromClass` "/Game/Game/Blueprint/BP_Endgame.BP_Endgame_C" (`KismetMathLibrary.MakeTransform` (0.0 0.0 0.0)) "AlwaysSpawn" "MultiplyWithRoot" null null))
  (`/Game/Game/Blueprint/BP_Endgame.Defeat` _returnvalue))

(event `StartHUD`
  (`self.HUD server`))

(event `HUD client`
  (if (`self.IsLocalController`)
    (bind _hud (`self.HUD`)
      (:`then`
        (`Widget.RemoveFromParent` _hud))
      (:`else`
        _))
    (bind _returnvalue (`|CreateWidget` "/Game/Game/HUD/Widget/WBP_HUD.WBP_HUD_C"))
    (bind _output_get (set `self.HUD` _returnvalue))
    (`/Game/Game/HUD/Widget/WBP_HUD.PlayFadeIn` _output_get)
    (bind _asbp_player_manager (cast `/Game/Game/Blueprint/BP_PlayerManager` (`self.K2_GetPawn` self))
      (:`then`
        (bind _output_get_2 (set `/Game/Game/Blueprint/BP_PlayerManager.HUD` _output_get _asbp_player_manager))
        (`UserWidget.AddToViewport` _output_get_2 0))
      (:`CastFailed`
        _))
    (`KismetSystemLibrary.K2_SetTimerDelegate` (delegate `DefeatServer`) 600.0)))

(event `DeathHUDServer`
  (if (`self.IsLocalController`)
    (bind _returnvalue (`|CreateWidget` "/Game/Game/HUD/Widget/WBP_Death.WBP_Death_C"))
    (`UserWidget.AddToViewport` _returnvalue 0)))

(fn `UserConstructionScript`)