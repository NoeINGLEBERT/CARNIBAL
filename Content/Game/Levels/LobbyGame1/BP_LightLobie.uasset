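; BP_LightLobie is a lobby light actor that moves a SpotLight continuously along a Spline path.
; Each Tick advances the travelled distance by SplineSpeed scaled by delta time, then places the light at that point in spline local space.
; The light keeps a fixed relative rotation instead of following the spline's direction.
; Once the distance passes the spline's length it resets to zero, looping the motion.
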(event `self.ReceiveTick`
  (params (DeltaSeconds :type "Float (single-precision)"))
  (bind _returnvalue_location (`KismetMathLibrary.BreakTransform` (`SplineComponent.GetTransformAtDistanceAlongSpline` (`self.Spline`) (`self.DistanceSpline`) "Local" false)))
  (set `self.DistanceSpline` (+ (* DeltaSeconds (`self.SplineSpeed`)) (`self.DistanceSpline`)))
  (`SceneComponent.K2_SetRelativeTransform` (`self.SpotLight`) (`KismetMathLibrary.MakeTransform` _returnvalue_location (struct :`Pitch` 250.0) (`SceneComponent.K2_GetComponentScale` (`self.SpotLight`))) false false)
  (if (> (`self.DistanceSpline`) (`SplineComponent.GetSplineLength` (`self.Spline`)))
    (set `self.DistanceSpline` 0.0)))

(fn `UserConstructionScript`)