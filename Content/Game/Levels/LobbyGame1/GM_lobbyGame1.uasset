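; Game mode for the LobbyGame1 level that creates the lobby UI and gives joining players an avatar.
; On BeginPlay it shows UI_PlayGame and creates UI_main, storing it without displaying it.
; Each new player joins a Controllers list, which is scanned to spawn and possess a BP_PlayerAvatar at index-named PlayerStarts for pawnless controllers.
; Logout removes the controller; a PublicConnections capacity check exists but never runs.
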(event `self.ReceiveBeginPlay`
  (bind _returnvalue (`|CreateWidget` "/Game/Game/Levels/LobbyGame1/UI_PlayGame.UI_PlayGame_C"))
  (`UserWidget.AddToPlayerScreen` _returnvalue 0)
  (bind _returnvalue_2 (`|CreateWidget` "/Game/Game/Levels/M/UI_main.UI_main_C"))
  (bind _asui_main (cast `/Game/Game/Levels/M/UI_main` _returnvalue_2))
  (set `self.As UI Main_0` _asui_main))

(event `self.K2_PostLogin`
  (params (NewPlayer :type "PlayerController Object Reference")))

(event `self.HandleStartingNewPlayer`
  (params (NewPlayer :type "PlayerController Object Reference"))
  (`KismetArrayLibrary.Array_AddUnique` (`self.Controllers`) NewPlayer)
  (for (_array_element _array_index) (`self.Controllers`)
    (if (== (`Controller.K2_GetPawn` _array_element) null)
      (bind _returnvalue (`|SpawnActorFromClass` "/Game/Game/Levels/LobbyGame1/BP_PlayerAvatar.BP_PlayerAvatar_C" (`self.GetTransform` (`self.K2_FindPlayerStart` _array_element (`KismetStringLibrary.Conv_IntToString` _array_index))) "Undefined" "MultiplyWithRoot" null null))
      (`Controller.Possess` _array_element _returnvalue))))

(event `self.K2_OnLogout`
  (params (ExitingController :type "Controller Object Reference"))
  (bind _asplayer_controller (cast `PlayerController` ExitingController))
  (`KismetArrayLibrary.Array_RemoveItem` (`self.Controllers`) _asplayer_controller))

(fn `UserConstructionScript`)