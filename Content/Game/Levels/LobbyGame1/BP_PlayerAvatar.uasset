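; BP_PlayerAvatar is the lobby player avatar that shows each player's Steam name on a widget name tag.
; Every tick, the locally controlled instance reads its Steam persona name and passes it to SetPlayerNameOnServeur, which sets CustomPlayerName.
; The variable's OnRep updates and unhides the tag, retrying by timer until the widget is valid.
; Its camera gets a fixed starting position, and CameraValue repositions it along Y.
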(event `CameraValue`
  (params (Value :type "Float (double-precision)"))
  (bind _result (`/Engine/EditorBlueprintResources/StandardMacros.NegateFloat` Value)
    (:`  `
      (`SceneComponent.K2_SetWorldLocation` (`self.Camera`) (`KismetMathLibrary.MakeVector` 0.0 _result) false false))))

(event `self.ReceiveBeginPlay`
  (`SceneComponent.K2_SetWorldLocation` (`self.Camera`) (0.0 -200.0 0.0) false false))

(event `self.ReceiveTick`
  (params (DeltaSeconds :type "Float (single-precision)"))
  (`self.SetUpLocat`))

(event `SetPlayerNameOnServeur`
  (params (CustomPlayerName :type Text))
  (set `self.CustomPlayerName` CustomPlayerName))

(fn `OnRep_CustomPlayerName`
  (bind _returnvalue (`WidgetComponent.GetWidget` (`self.Widget`)))
  (`/Engine/EditorBlueprintResources/StandardMacros.IsValid` _returnvalue
    (:`Is Valid`
      (bind _asui_player_name_tag (cast `/Game/Game/HUD/Widget/UI_PlayerNameTag` _returnvalue))
      (`/Game/Game/HUD/Widget/UI_PlayerNameTag.SetPlayerName` _asui_player_name_tag (`self.CustomPlayerName`))
      (`SceneComponent.SetHiddenInGame` (`self.Widget`) false false))
    (:`Is Not Valid`
      (`KismetSystemLibrary.K2_SetTimer` null "OnRep_CustomPlayerName" 0.1))))

(fn `SetUpLocat`
  (if (`self.IsLocallyControlled`)
    (bind _returnvalue (`AdvancedSteamFriendsLibrary.GetSteamPersonaName` (`AdvancedSessionsLibrary.GetUniqueNetIDFromPlayerState` (`Controller.PlayerState` (`self.GetController`)))))
    (`self.SetPlayerNameOnServeur` (`KismetTextLibrary.Conv_StringToText` _returnvalue))))

(fn `UserConstructionScript`)