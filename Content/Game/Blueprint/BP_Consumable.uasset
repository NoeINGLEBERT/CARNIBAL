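; Consumable actor that a BP_PlayerManager of sufficient Level eats by overlapping it with its Box, once EatDelay has run out.
; The overlap stores the eater, distance and time, and aims the eater's TargetArrow at the Sphere.
; Tick then draws the Sphere toward the eater's visual Box along that arrow, timed by relative speed, while blending rotation.
; Within close range it plays a crunch sound, calls the empty Consumed event and destroys itself.
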(event `self.ReceiveTick`
  (params (DeltaSeconds :type "Float (single-precision)"))
  (bind _sphere (`self.Sphere`))
  (bind _killerref (`self.KillerRef`))
  (bind _box (`/Game/Game/Blueprint/BP_PlayerVisuals.Box` (`/Game/Game/Blueprint/BP_PlayerManager.Visuals` (`self.KillerRef`))))
  (bind _returnvalue (+ (`SceneComponent.K2_GetComponentLocation` _box) (* (`SceneComponent.GetForwardVector` _box) 1.0)))
  (set `self.EatDelay` (- (`self.EatDelay`) DeltaSeconds))
  (`|ExecutionSequence`
    (:`then_1`
      (if (!= (`self.KillerRef`) null)
        (`SceneComponent.K2_SetWorldLocation` (`self.Sphere`) (`|EaseFunction` "Linear" (- 1.0 (`KismetMathLibrary.FClamp` (/ (- (`GameplayStatics.GetTimeSeconds`) (`self.DeathTimeStamp`)) (/ (`self.KillerDistance`) (- (`KismetMathLibrary.Dot_VectorVector` (`self.GetActorForwardVector` _killerref) (`MovementComponent.Velocity` (`Character.CharacterMovement` _killerref))) (`self.DeathSpeed`)))))) _returnvalue (+ _returnvalue (* (`SceneComponent.GetForwardVector` (`/Game/Game/Blueprint/BP_PlayerVisuals.TargetArrow` (`/Game/Game/Blueprint/BP_PlayerManager.Visuals` (`self.KillerRef`)))) (`self.KillerDistance`)))) false false)
        (`SceneComponent.K2_SetWorldRotation` _sphere (`|EaseFunction` "Linear" 0.2 (`SceneComponent.K2_GetComponentRotation` _sphere) (`SceneComponent.K2_GetComponentRotation` (`/Game/Game/Blueprint/BP_PlayerVisuals.Box` (`/Game/Game/Blueprint/BP_PlayerManager.Visuals` (`self.KillerRef`))))) false false)
        (if (< (`KismetMathLibrary.Vector_Distance` (`SceneComponent.K2_GetComponentLocation` (`self.Sphere`)) (`SceneComponent.K2_GetComponentLocation` (`/Game/Game/Blueprint/BP_PlayerVisuals.Box` (`/Game/Game/Blueprint/BP_PlayerManager.Visuals` (`self.KillerRef`))))) 20.0)
          (`/Engine/EditorBlueprintResources/StandardMacros.DoOnce` false
            (:`Completed`
              (`self.LazyFix`)
              (`self.K2_DestroyActor`))))))))

(event `LazyFix`
  (`FMODBlueprintStatics.PlayEventAttached` "/Game/FMOD/Events/SFX_Vehicle/Event_Vehicle_Crunch.Event_Vehicle_Crunch" (`/Game/Game/Blueprint/BP_PlayerManager.Box` (`self.KillerRef`)) "None" (0.0 0.0 0.0) "KeepRelativeOffset")
  (`self.Consumed`))

(event `Consumed`)

(event `self.Box.OnComponentBeginOverlap`
  (params (OverlappedComponent :type "PrimitiveComponent Object Reference") (OtherActor :type "Actor Object Reference") (OtherComp :type "PrimitiveComponent Object Reference") (OtherBodyIndex :type Integer) (bFromSweep :type Boolean) (SweepResult :type "HitResult Structure (by ref)"))
  (if (not (> (`self.EatDelay`) 0.0))
    (bind _asbp_player_manager (cast `/Game/Game/Blueprint/BP_PlayerManager` OtherActor))
    (if (and (== (`/Game/Game/Blueprint/BP_PlayerManager.Box` _asbp_player_manager) OtherComp) (>= (`/Game/Game/Blueprint/BP_PlayerManager.Level` _asbp_player_manager) (`self.MinSizeToEat`)))
      (bind _output_get (set `self.KillerRef` _asbp_player_manager))
      (bind _box (`/Game/Game/Blueprint/BP_PlayerVisuals.Box` (`/Game/Game/Blueprint/BP_PlayerManager.Visuals` _output_get)))
      (bind _returnvalue (- (`SceneComponent.K2_GetComponentLocation` (`self.Sphere`)) (+ (`SceneComponent.K2_GetComponentLocation` _box) (* (`SceneComponent.GetForwardVector` _box) 1.0))))
      (`SceneComponent.K2_SetWorldRotation` (`/Game/Game/Blueprint/BP_PlayerVisuals.TargetArrow` (`/Game/Game/Blueprint/BP_PlayerManager.Visuals` (`self.KillerRef`))) (`KismetMathLibrary.MakeRotFromX` _returnvalue) false false)
      (set `self.KillerDistance` (`KismetMathLibrary.VSize` _returnvalue))
      (set `self.DeathTimeStamp` (`GameplayStatics.GetTimeSeconds`))
      (set `self.DeathSpeed` (`KismetMathLibrary.VSize` (`SceneComponent.GetForwardVector` (`/Game/Game/Blueprint/BP_PlayerVisuals.Box` (`/Game/Game/Blueprint/BP_PlayerManager.Visuals` (`self.KillerRef`)))))))))

(fn `UserConstructionScript`)