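; BP_Debris is a debris actor that flies under simple scripted gravity until it lands, using no physics simulation in its graph.
; Each Tick, it line-traces vertically over the frame's Z movement; on a hit it snaps there, stops updating and plays an attached debris audio event.
; Otherwise it moves by Velocity times delta time, after subtracting a fixed downward step that is not delta-scaled, so gravity varies with frame rate.
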(event `self.ReceiveTick`
  (params (DeltaSeconds :type "Float (single-precision)"))
  (bind _returnvalue (`self.K2_GetActorLocation`))
  (`parent.ReceiveTick` DeltaSeconds)
  (if (not (`self.OnGround`))
    (bind (_outhit _returnvalue_2) (`KismetSystemLibrary.LineTraceSingle` _returnvalue (+ _returnvalue (`KismetMathLibrary.MakeVector` 0.0 0.0 (* (.z (`self.Velocity`)) (`GameplayStatics.GetWorldDeltaSeconds`)))) "TraceTypeQuery3"))
    (if _returnvalue_2
      (`self.K2_SetActorLocation` (`.Location` (`GameplayStatics.BreakHitResult` _outhit)))
      (set `self.OnGround` true)
      (`FMODBlueprintStatics.PlayEventAttached` "/Game/FMOD/Events/SFX_Other/Event_Debris.Event_Debris" (`self.Cube`) "None" (0.0 0.0 0.0) "KeepRelativeOffset")
      (else
        (bind _output_get (set `self.Velocity` (- (`self.Velocity`) (0.0 0.0 50.0))))
        (`self.K2_SetActorLocation` (+ (`self.K2_GetActorLocation`) (* _output_get (`GameplayStatics.GetWorldDeltaSeconds`))))))))

(fn `UserConstructionScript`
  (`parent.UserConstructionScript`))