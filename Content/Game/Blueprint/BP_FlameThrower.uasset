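; BP_FlameThrower is a toggled weapon that emits flames and spawns damage hitboxes while active.
; Each Shot call flips firing, switching the Niagara effect, looping hitbox timer, attached sound and the manager's fuel-loss rate.
; Spawned BP_FlameThrowerHitbox actors launch along the arrow, inheriting the movement component's velocity, the owning manager and a timestamp.
; Tick feeds that same velocity into the Niagara effect so flames follow the user's motion.
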(event `SpawnHitbox`
  (bind _arrow (`self.Arrow`))
  (bind (_returnvalue_location _returnvalue_rotation) (`KismetMathLibrary.BreakTransform` (`SceneComponent.K2_GetComponentToWorld` _arrow)))
  (bind _movementref (`self.MovementRef`)
    (:`then`
      (bind _returnvalue (`|SpawnActorFromClass` "/Game/Game/Blueprint/BP_FlameThrowerHitbox.BP_FlameThrowerHitbox_C" (`KismetMathLibrary.MakeTransform` _returnvalue_location _returnvalue_rotation) "Undefined" "MultiplyWithRoot" null null))
      (set `/Game/Game/Blueprint/BP_FlameThrowerHitbox.OwnManager` (`self.OwnManager`) _returnvalue)
      (set `/Game/Game/Blueprint/BP_FlameThrowerHitbox.Velocity` (+ (* (`SceneComponent.GetForwardVector` _arrow) 2000.0) (`MovementComponent.Velocity` _movementref)) _returnvalue)
      (set `/Game/Game/Blueprint/BP_FlameThrowerHitbox.SpawnTimeStamp` (`GameplayStatics.GetTimeSeconds`) _returnvalue))
    (:`else`)))

(event `self.Shot`
  (params (Movement :type "CharacterMovementComponent Object Reference") (Manager :type "/Game/Game/Blueprint/BP_PlayerManager Object Reference"))
  (bind _niagara (`self.Niagara`))
  (set `self.MovementRef` Movement)
  (set `self.OwnManager` Manager)
  (`/Engine/EditorBlueprintResources/StandardMacros.FlipFlop`
    (:`A`
      (`ActorComponent.Activate` _niagara false)
      (bind _returnvalue (`KismetSystemLibrary.K2_SetTimerDelegate` (delegate `SpawnHitbox`) 0.1 true))
      (set `self.SpawnTimer` _returnvalue)
      (set `/Game/Game/Blueprint/BP_PlayerManager.FuelLoss` -0.2 (`self.OwnManager`))
      (bind _returnvalue_2 (`FMODBlueprintStatics.PlayEventAttached` "/Game/FMOD/Events/SFX_Weapons/Event_Weapon_Flamethrower.Event_Weapon_Flamethrower" (`self.StaticMesh`) "None" (0.0 0.0 0.0) "KeepRelativeOffset"))
      (set `self.SFX` _returnvalue_2))
    (:`B`
      (`ActorComponent.Deactivate` _niagara)
      (`KismetSystemLibrary.K2_ClearAndInvalidateTimerHandle` (`self.SpawnTimer`))
      (set `/Game/Game/Blueprint/BP_PlayerManager.FuelLoss` -0.02 (`self.OwnManager`))
      (`FMODAudioComponent.Stop` (`self.SFX`)))))

(event `self.ReceiveTick`
  (params (DeltaSeconds :type "Float (single-precision)"))
  (bind _movementref (`self.MovementRef`)
    (:`then`
      (`NiagaraComponent.SetNiagaraVariableVec3` (`self.Niagara`) "InitialVelocity" (`MovementComponent.Velocity` _movementref)))
    (:`else`)))

(fn `UserConstructionScript`
  (`parent.UserConstructionScript`))