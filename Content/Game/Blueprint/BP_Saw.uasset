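; BP_Saw is a saw hazard that deals damage to any BP_PlayerManager it hits.
; Each Tick spins StaticMesh and eases StaticMesh2 toward a direction derived from the actor's right vector, in the plane of StaticMesh.
; StaticMesh2's alignment with actor forward sets StaticMesh's X offset, and Bras2 rotates to track StaticMesh, like a procedural linkage.
; The attached saw sound starts once, on the first Tick.
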(event `self.ReceiveTick`
  (params (DeltaSeconds :type "Float (single-precision)"))
  (bind _staticmesh (`self.StaticMesh`))
  (bind _returnvalue (`SceneComponent.GetUpVector` (`self.StaticMesh`)))
  (bind _returnvalue_2 (`SceneComponent.GetUpVector` (`self.StaticMesh`)))
  (`parent.ReceiveTick` DeltaSeconds)
  (`SceneComponent.K2_SetWorldRotation` (`self.StaticMesh2`) (`|EaseFunction` "Linear" 0.1 (`KismetMathLibrary.MakeRotFromYZ` (`KismetMathLibrary.ProjectVectorOnToPlane` (`SceneComponent.GetRightVector` (`self.StaticMesh2`)) _returnvalue) _returnvalue) (`KismetMathLibrary.MakeRotFromXZ` (`KismetMathLibrary.NegateVector` (`self.GetActorRightVector`)) _returnvalue)) false false)
  (`SceneComponent.K2_SetRelativeLocation` (`self.StaticMesh`) (`KismetMathLibrary.MakeVector` (`KismetMathLibrary.MapRangeClamped` (`KismetMathLibrary.Dot_VectorVector` (`SceneComponent.GetRightVector` (`self.StaticMesh2`)) (`self.GetActorForwardVector`)) 0.0 1.0 0.0 357.0) -6.0 42.5) false false)
  (`SceneComponent.K2_SetWorldRotation` (`self.bras_2`) (`KismetMathLibrary.MakeRotFromYZ` (`KismetMathLibrary.ProjectVectorOnToPlane` (- (`SceneComponent.K2_GetComponentLocation` (`self.StaticMesh`)) (`SceneComponent.K2_GetComponentLocation` (`self.bras_2`))) _returnvalue_2) _returnvalue_2) false false)
  (`SceneComponent.K2_SetRelativeRotation` _staticmesh (`KismetMathLibrary.ComposeRotators` (`SceneComponent.RelativeRotation` _staticmesh) (struct :`Yaw` 10.0)) false false)
  (`/Engine/EditorBlueprintResources/StandardMacros.DoOnce` false
    (:`Completed`
      (`FMODBlueprintStatics.PlayEventAttached` "/Game/FMOD/Events/SFX_Weapons/Event_Weapon_Saw.Event_Weapon_Saw" (`self.StaticMesh`) "None" (0.0 0.0 0.0) "KeepRelativeOffset" true))))

(event `self.Hit`
  (params (OtherActor :type "Actor Object Reference"))
  (bind _asbp_player_manager (cast `/Game/Game/Blueprint/BP_PlayerManager` OtherActor))
  (`/Game/Game/Blueprint/BP_PlayerManager.TakeDamage` _asbp_player_manager 3))

(fn `UserConstructionScript`
  (`parent.UserConstructionScript`))