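; BP_FlameThrowerHitbox is a short-lived flamethrower damage volume that moves along its velocity while its sphere grows with age.
; Overlapping player managers other than its owner track it in their OverlappedFlame lists, while overlapping oil is stored locally.
; Each tick, LitOil traces from the flame center toward each oil's horizontally offset near edge, limited to the flame radius, and burns that oil on any blocking hit.
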(event `self.ReceiveTick`
  (params (DeltaSeconds :type "Float (single-precision)"))
  (bind _returnvalue (- (`GameplayStatics.GetTimeSeconds`) (`self.SpawnTimeStamp`)))
  (`self.K2_SetActorLocation` (+ (* DeltaSeconds (`self.Velocity`)) (`self.K2_GetActorLocation`)))
  (`SphereComponent.SetSphereRadius` (`self.Sphere`) (`KismetMathLibrary.MapRangeClamped` _returnvalue 0.0 2.0 0.0 500.0) true)
  (if (> _returnvalue 1.575)
    (`self.K2_DestroyActor`)
    (else
      (`self.LitOil`))))

(event `self.Sphere.OnComponentBeginOverlap`
  (params (OverlappedComponent :type "PrimitiveComponent Object Reference") (OtherActor :type "Actor Object Reference") (OtherComp :type "PrimitiveComponent Object Reference") (OtherBodyIndex :type Integer) (bFromSweep :type Boolean) (SweepResult :type "HitResult Structure (by ref)"))
  (bind _ownmanager (`self.OwnManager`))
  (bind _asbp_oil (cast `/Game/Game/Blueprint/BP_Oil` OtherActor)
    (:`then`
      (`KismetArrayLibrary.Array_AddUnique` (`self.OverlappedOil`) _asbp_oil))
    (:`CastFailed`
      (if (and (!= OtherActor _ownmanager) (!= _ownmanager null))
        (bind _asbp_player_manager (cast `/Game/Game/Blueprint/BP_PlayerManager` OtherActor))
        (`KismetArrayLibrary.Array_AddUnique` (`/Game/Game/Blueprint/BP_PlayerManager.OverlappedFlame` _asbp_player_manager) self)))))

(event `self.Sphere.OnComponentEndOverlap`
  (params (OverlappedComponent :type "PrimitiveComponent Object Reference") (OtherActor :type "Actor Object Reference") (OtherComp :type "PrimitiveComponent Object Reference") (OtherBodyIndex :type Integer))
  (bind _ownmanager (`self.OwnManager`))
  (bind _asbp_oil (cast `/Game/Game/Blueprint/BP_Oil` OtherActor)
    (:`then`
      (`KismetArrayLibrary.Array_RemoveItem` (`self.OverlappedOil`) _asbp_oil))
    (:`CastFailed`
      (if (and (!= OtherActor _ownmanager) (!= _ownmanager null))
        (bind _asbp_player_manager (cast `/Game/Game/Blueprint/BP_PlayerManager` OtherActor))
        (`KismetArrayLibrary.Array_RemoveItem` (`/Game/Game/Blueprint/BP_PlayerManager.OverlappedFlame` _asbp_player_manager) self)))))

(fn `LitOil`
  (bind _sphere (`self.Sphere`))
  (bind _returnvalue (`SceneComponent.K2_GetComponentLocation` _sphere))
  (for _array_element (`self.OverlappedOil`)
    (if (`KismetSystemLibrary.IsValid` _array_element)
      (bind _returnvalue_2 (`self.K2_GetActorLocation` _array_element))
      (bind (_returnvalue_x _returnvalue_y) (`KismetMathLibrary.BreakVector` (`KismetMathLibrary.Normal` (- _returnvalue_2 _returnvalue))))
      (bind (_outhit _returnvalue_3) (`KismetSystemLibrary.LineTraceSingle` :`Start` _returnvalue :`End` (+ (* (`KismetMathLibrary.Normal` (- (- _returnvalue_2 (* (`KismetMathLibrary.MakeVector` _returnvalue_x _returnvalue_y) (`SphereComponent.SphereRadius` (`/Game/Game/Blueprint/BP_Oil.Sphere` _array_element)))) _returnvalue)) (`SphereComponent.SphereRadius` _sphere)) _returnvalue) :`TraceChannel` "TraceTypeQuery3" :`DrawDebugType` "ForOneFrame"))
      (if _returnvalue_3
        (`/Game/Game/Blueprint/BP_Oil.Burn` _array_element)))))

(fn `UserConstructionScript`)