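; Melee attachment actor that detects hits through a Box overlap and limits how often each target can be hit.
; An overlapping actor other than OwnManager that has no active cooldown is added to the HitCooldowns map and passed to Hit.
; Tick rebuilds that map every frame with decremented timers, dropping expired entries.
; Hit is empty here, and re-hits require a new begin-overlap.
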(event `self.ReceiveTick`
  (params (DeltaSeconds :type "Float (single-precision)"))
  (set `self.HitCooldownsTemp` (`|MakeMap`))
  (bind _values (`BlueprintMapLibrary.Map_Values` (`self.HitCooldowns`)))
  (for (_array_element _array_index) _values
    (bind _returnvalue (- _array_element DeltaSeconds))
    (if (> _returnvalue 0.0)
      (bind _keys (`BlueprintMapLibrary.Map_Keys` (`self.HitCooldowns`)))
      (`BlueprintMapLibrary.Map_Add` (`self.HitCooldownsTemp`) (`|GetArrayItem` _keys _array_index) _returnvalue)))
  (set `self.HitCooldowns` (`self.HitCooldownsTemp`)))

(event `self.Box.OnComponentBeginOverlap`
  (params (OverlappedComponent :type "PrimitiveComponent Object Reference") (OtherActor :type "Actor Object Reference") (OtherComp :type "PrimitiveComponent Object Reference") (OtherBodyIndex :type Integer) (bFromSweep :type Boolean) (SweepResult :type "HitResult Structure (by ref)"))
  (bind _keys (`BlueprintMapLibrary.Map_Keys` (`self.HitCooldowns`)))
  (if (and (!= OtherActor (`self.OwnManager`)) (not (`KismetArrayLibrary.Array_Contains` _keys OtherActor)))
    (`BlueprintMapLibrary.Map_Add` (`self.HitCooldowns`) OtherActor (`self.Cooldown`))
    (`self.Hit` OtherActor)))

(event `Hit`
  (params (OtherActor :type "Actor Object Reference")))

(fn `UserConstructionScript`)