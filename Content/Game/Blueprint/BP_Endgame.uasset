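; BP_Endgame handles the end of a match, with Victory and Defeat events that play the win or overtime level sequence.
; Both events also hide the HUD of every BP_PlayerManager while their cinematic plays.
; When either sequence finishes, a shared Credits event shows WBP_Credits, waits on a fixed delay, then server-travels to LobbyGame1 through a console command.
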(event `Victory`
  (bind (_outactor _returnvalue) (`LevelSequencePlayer.CreateLevelSequencePlayer` "/Game/Game/Anim/LevelSequence/LC_EndGameWin.LC_EndGameWin"))
  (add `MovieSceneSequencePlayer.OnFinished` _returnvalue (delegate `Credits`))
  (`MovieSceneSequencePlayer.Play` _returnvalue)
  (bind _outactors (`GameplayStatics.GetAllActorsOfClass` "/Game/Game/Blueprint/BP_PlayerManager.BP_PlayerManager_C"))
  (for _array_element _outactors
    (set `Widget.Visibility` "Hidden" (`/Game/Game/Blueprint/BP_PlayerManager.HUD` _array_element))))

(event `Credits`
  (bind _returnvalue (`|CreateWidget` "/Game/Game/HUD/Widget/WBP_Credits.WBP_Credits_C"))
  (`UserWidget.AddToViewport` _returnvalue 0)
  (`KismetSystemLibrary.Delay` 25.0)
  (`KismetSystemLibrary.ExecuteConsoleCommand` "serverTravel LobbyGame1" null))

(event `Defeat`
  (bind (_outactor _returnvalue) (`LevelSequencePlayer.CreateLevelSequencePlayer` "/Game/Game/Anim/LevelSequence/LC_EndGameOvertime.LC_EndGameOvertime"))
  (add `MovieSceneSequencePlayer.OnFinished` _returnvalue (delegate `Credits`))
  (`MovieSceneSequencePlayer.Play` _returnvalue)
  (bind _outactors (`GameplayStatics.GetAllActorsOfClass` "/Game/Game/Blueprint/BP_PlayerManager.BP_PlayerManager_C"))
  (for _array_element _outactors
    (set `Widget.Visibility` "Hidden" (`/Game/Game/Blueprint/BP_PlayerManager.HUD` _array_element))))

(fn `UserConstructionScript`)