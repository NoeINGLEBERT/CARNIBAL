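; BP_VacuumCleaner is a vacuum actor that sucks up BP_Oil and grants fuel to its owning manager.
; Hitting new oil starts a sound and the CollectOil timeline, which moves the oil toward the vacuum while scaling its material radius and collision sphere.
; Leaving the Box starts a one-second grace delay before the oil is released, but the timeline still finishes and awards fuel.
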(event `self.Hit`
  (params (OtherActor :type "Actor Object Reference"))
  (bind _asbp_oil (cast `/Game/Game/Blueprint/BP_Oil` OtherActor))
  (set `self.OutOfRange` false)
  (if (!= _asbp_oil (`self.Oil`))
    (bind _output_get (set `self.Oil` _asbp_oil))
    (bind _returnvalue (`MaterialInstanceDynamic.K2_GetScalarParameterValue` (`/Game/Game/Blueprint/BP_Oil.DynamicMaterial` _output_get) "Radius"))
    (set `self.StartRadius` _returnvalue)
    (set `self.StartLocation` (`self.K2_GetActorLocation` (`self.Oil`)))
    (`self.CustomEvent`)))

(event `CustomEvent`
  (bind _returnvalue (`FMODBlueprintStatics.PlayEventAttached` "/Game/FMOD/Events/SFX_Weapons/Event_Weapon_Vacuum.Event_Weapon_Vacuum" (`self.StaticMesh`) "None" (0.0 0.0 0.0) "KeepRelativeOffset"))
  (set `self.SFX` _returnvalue)
  (bind (_direction _oilleft) (`Timeline|CollectOil` :!via `PlayFromStart`)
    (:`Update`
      (if (and (`self.OutOfRange`) (< (`self.Delay`) 0.0))
        (set `self.Oil` null)
        (else
          (bind _oil (`self.Oil`)
            (:`then`
              (`self.K2_SetActorLocation` _oil (`|EaseFunction` "Linear" _oilleft (`self.K2_GetActorLocation`) (`self.StartLocation`)) false false)
              (bind _returnvalue_2 (* _oilleft (`self.StartRadius`)))
              (`MaterialInstanceDynamic.SetScalarParameterValue` (`/Game/Game/Blueprint/BP_Oil.DynamicMaterial` _oil) "Radius" _returnvalue_2)
              (`SphereComponent.SetSphereRadius` (`/Game/Game/Blueprint/BP_Oil.Sphere` _oil) _returnvalue_2 true)
              (set `self.Delay` (- (`self.Delay`) (`GameplayStatics.GetWorldDeltaSeconds`))))
            (:`else`)))))
    (:`Finished`
      (bind _ownmanager (`self.OwnManager`)
        (:`then`
          (`/Game/Game/Blueprint/BP_PlayerManager.FuelUpdate` _ownmanager 5.0)
          (`FMODAudioComponent.Stop` (`self.SFX`)))
        (:`else`)))))

(event `self.Box.OnComponentEndOverlap`
  (params (OverlappedComponent :type "PrimitiveComponent Object Reference") (OtherActor :type "Actor Object Reference") (OtherComp :type "PrimitiveComponent Object Reference") (OtherBodyIndex :type Integer))
  (if (== OtherActor (`self.Oil`))
    (set `self.OutOfRange` true)
    (set `self.Delay` 1.0)))

(fn `UserConstructionScript`
  (`parent.UserConstructionScript`))