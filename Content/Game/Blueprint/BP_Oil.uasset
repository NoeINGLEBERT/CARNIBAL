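; BP_Oil is an oil puddle that grows over time, cuts player control on contact, and can catch fire.
; A timeline drives one radius shared by the decal material, overlap sphere and Niagara effect.
; Overlaps track neighboring puddles and set the player's control value and FMOD on-gas parameter.
; Burning plays fire audio and effects, ignites neighbors after a short delay, and animates the radius before self-destruction.
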(event `self.ReceiveTick`
  (params (DeltaSeconds :type "Float (single-precision)"))
  (`/Engine/EditorBlueprintResources/StandardMacros.DoOnce` false
    (:`Completed`
      (bind _returnvalue (`KismetMaterialLibrary.CreateDynamicMaterialInstance` "/Game/Game/Materials/MI_Oil.MI_Oil"))
      (bind _output_get (set `self.DynamicMaterial` _returnvalue))
      (`DecalComponent.SetDecalMaterial` (`self.Decal`) _output_get)
      (bind (_direction _oilradius) (`Timeline|TimelineRadius` :!via `PlayFromStart` :!label _label)
        (:`Update`
          (`self.UpdateRadius` _oilradius))))))

(event `Burn`
  (`/Engine/EditorBlueprintResources/StandardMacros.DoOnce` false
    (:`Completed`
      (bind _returnvalue (`FMODBlueprintStatics.PlayEventAttached` "/Game/FMOD/Events/SFX_Weapons/Event_Weapon_Gasoline_Fire.Event_Weapon_Gasoline_Fire" (`self.Sphere`) "None" (0.0 0.0 0.0) "KeepRelativeOffset"))
      (`KismetSystemLibrary.K2_SetTimerDelegate` (delegate `Propagate`) 0.05)
      (`ActorComponent.Activate` (`self.Niagara`) false)
      (`|ExecutionSequence`
        (:`then_0`
          (goto _label :!via `Stop`))
        (:`then_1`
          (bind (_direction _radius) (`Timeline|TimelineBurn` :`NewTime` (* (- 1.0 (stale `self.ReceiveTick` _oilradius)) 5.0) :!via `SetNewTime` :!label _label_2)
            (:`Update`
              (`self.UpdateRadius` _radius))
            (:`Finished`
              (`FMODAudioComponent.Stop` _returnvalue)
              (`ActorComponent.Deactivate` (`self.Niagara`))
              (`KismetSystemLibrary.Delay` 1.0)
              (`self.K2_DestroyActor`))))
        (:`then_2`
          (goto _label_2))))))

(event `Propagate`
  (for _array_element (`self.OverlappedOil`)
    (`self.Burn` _array_element)))

(event `self.Sphere.OnComponentBeginOverlap`
  (params (OverlappedComponent :type "PrimitiveComponent Object Reference") (OtherActor :type "Actor Object Reference") (OtherComp :type "PrimitiveComponent Object Reference") (OtherBodyIndex :type Integer) (bFromSweep :type Boolean) (SweepResult :type "HitResult Structure (by ref)"))
  (bind _asbp_player_manager (cast `/Game/Game/Blueprint/BP_PlayerManager` OtherActor)
    (:`then`
      (set `/Game/Game/Blueprint/BP_PlayerManager.ControlValue` 0.0 _asbp_player_manager)
      (`KismetArrayLibrary.Array_AddUnique` (`/Game/Game/Blueprint/BP_PlayerManager.OverlappedOil` _asbp_player_manager) self)
      (`FMODAudioComponent.SetParameter` (`/Game/Game/Blueprint/BP_PlayerManager.FModMovement` _asbp_player_manager) "Param_IsOnGas" 1.0))
    (:`CastFailed`
      (bind _asbp_oil (cast `/Game/Game/Blueprint/BP_Oil` OtherActor))
      (`KismetArrayLibrary.Array_AddUnique` (`self.OverlappedOil`) _asbp_oil))))

(event `self.Sphere.OnComponentEndOverlap`
  (params (OverlappedComponent :type "PrimitiveComponent Object Reference") (OtherActor :type "Actor Object Reference") (OtherComp :type "PrimitiveComponent Object Reference") (OtherBodyIndex :type Integer))
  (bind _asbp_player_manager (cast `/Game/Game/Blueprint/BP_PlayerManager` OtherActor)
    (:`then`
      (bind _overlappedoil (`/Game/Game/Blueprint/BP_PlayerManager.OverlappedOil` _asbp_player_manager))
      (`KismetArrayLibrary.Array_RemoveItem` _overlappedoil self)
      (if (== (`KismetArrayLibrary.Array_Length` _overlappedoil) 0)
        (set `/Game/Game/Blueprint/BP_PlayerManager.ControlValue` 1.0 _asbp_player_manager)
        (`FMODAudioComponent.SetParameter` (`/Game/Game/Blueprint/BP_PlayerManager.FModMovement` _asbp_player_manager) "Param_IsOnGas" 0.0)))
    (:`CastFailed`
      (bind _asbp_oil (cast `/Game/Game/Blueprint/BP_Oil` OtherActor))
      (`KismetArrayLibrary.Array_RemoveItem` (`self.OverlappedOil`) _asbp_oil))))

(fn `UpdateRadius`
  (params (Percent :type "Float (double-precision)"))
  (bind _returnvalue (* Percent 750.0))
  (`MaterialInstanceDynamic.SetScalarParameterValue` (`self.DynamicMaterial`) "Radius" _returnvalue)
  (`SphereComponent.SetSphereRadius` (`self.Sphere`) _returnvalue true)
  (`FXSystemComponent.SetFloatParameter` (`self.Niagara`) "Radius" _returnvalue)
  (`FXSystemComponent.SetFloatParameter` (`self.Niagara`) "SpawnRate" (* (`KismetMathLibrary.MultiplyMultiply_FloatFloat` Percent 3.0) 36000.0)))

(fn `UserConstructionScript`)