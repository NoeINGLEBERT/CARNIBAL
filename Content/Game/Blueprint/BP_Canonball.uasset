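; BP_Canonball is a cannonball projectile that damages players other than the one stored in OwnManager.
; Each tick it moves by its Velocity without sweeping and destroys itself once it drops below a fixed height.
; When its sphere overlaps another BP_PlayerManager, it applies small random damage, plays a cannon-hit audio event at its location and destroys itself.
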(event `self.ReceiveTick`
  (params (DeltaSeconds :type "Float (single-precision)"))
  (bind _returnvalue (+ (* DeltaSeconds (`self.Velocity`)) (`self.K2_GetActorLocation`)))
  (`self.K2_SetActorLocation` _returnvalue)
  (if (< (.z _returnvalue) -100.0)
    (`self.K2_DestroyActor`)))

(event `self.Sphere.OnComponentBeginOverlap`
  (params (OverlappedComponent :type "PrimitiveComponent Object Reference") (OtherActor :type "Actor Object Reference") (OtherComp :type "PrimitiveComponent Object Reference") (OtherBodyIndex :type Integer) (bFromSweep :type Boolean) (SweepResult :type "HitResult Structure (by ref)"))
  (bind _ownmanager (`self.OwnManager`))
  (if (and (!= OtherActor _ownmanager) (!= _ownmanager null))
    (bind _asbp_player_manager (cast `/Game/Game/Blueprint/BP_PlayerManager` OtherActor))
    (`/Game/Game/Blueprint/BP_PlayerManager.TakeDamage` _asbp_player_manager (`KismetMathLibrary.RandomIntegerInRange` 2 3))
    (`FMODBlueprintStatics.PlayEventAtLocation` "/Game/FMOD/Events/SFX_Vehicle/Event_Vehicle_Hit_Cannon.Event_Vehicle_Hit_Cannon" (`self.GetTransform`))
    (`self.K2_DestroyActor`)))

(fn `UserConstructionScript`)