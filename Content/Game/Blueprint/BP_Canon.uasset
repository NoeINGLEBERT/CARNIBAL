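; BP_Canon is a cannon weapon that fires BP_Canonball projectiles at the cost of Scrap.
; Its Shot event requires a minimum Scrap on the passed-in Manager, deducts one, and plays an attached cannon sound event.
; It spawns the ball at the Arrow component, assigns the Manager as owner, and adds the Movement's velocity to a fixed forward launch speed so shots inherit motion.
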(event `self.Shot`
  (params (Movement :type "CharacterMovementComponent Object Reference") (Manager :type "/Game/Game/Blueprint/BP_PlayerManager Object Reference"))
  (if (>= (`/Game/Game/Blueprint/BP_PlayerManager.Scrap` Manager) 11)
    (`/Game/Game/Blueprint/BP_PlayerManager.ScrapUpdate` Manager -1)
    (`FMODBlueprintStatics.PlayEventAttached` "/Game/FMOD/Events/SFX_Weapons/Event_Weapon_Cannon.Event_Weapon_Cannon" (`self.StaticMesh`) "None" (0.0 0.0 0.0) "KeepRelativeOffset")
    (bind _returnvalue (`|SpawnActorFromClass` "/Game/Game/Blueprint/BP_Canonball.BP_Canonball_C" (`SceneComponent.K2_GetComponentToWorld` (`self.Arrow`)) "Undefined" "MultiplyWithRoot" null null))
    (set `/Game/Game/Blueprint/BP_Canonball.OwnManager` Manager _returnvalue)
    (set `/Game/Game/Blueprint/BP_Canonball.Velocity` (+ (`MovementComponent.Velocity` Movement) (* (`SceneComponent.GetForwardVector` (`self.Arrow`)) 10000.0)) _returnvalue)))

(fn `UserConstructionScript`
  (`parent.UserConstructionScript`))