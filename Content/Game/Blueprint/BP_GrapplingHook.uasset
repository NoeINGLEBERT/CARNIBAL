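; Grappling hook actor that fires a harpoon to reel another player toward its owner, or the owner toward whatever else it hits.
; Shot toggles firing and release; launch velocity inherits player movement and slows for nearby, well-aimed targets.
; Tick flies the harpoon with manual gravity, then eases the pulled player by teleport, passing displacement to that player's attached hooks.
; Sphere overlap selects pull mode, aligning world hits with a Level-scaled trace.
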(event `self.Shot`
  (params (Movement :type "CharacterMovementComponent Object Reference") (Manager :type "/Game/Game/Blueprint/BP_PlayerManager Object Reference"))
  (bind _returnvalue (`self.K2_GetActorLocation` (`self.OwnManager`)))
  (bind _returnvalue_2 (+ (* (`SceneComponent.GetForwardVector` (`self.Arrow`)) 10000.0) (0.0 0.0 500.0)))
  (set `self.OwnManager` Manager)
  (bind _output_get (set `self.MovementRef` Movement))
  (bind _closesttarget (`/Game/Game/Blueprint/BP_PlayerVisuals.ClosestTarget` (`/Game/Game/Blueprint/BP_PlayerManager.Visuals` Manager))
    (:`then`
      (bind _returnvalue_3 (`self.K2_GetActorLocation` _closesttarget))
      (bind _returnvalue_4 (`KismetMathLibrary.Vector_Distance` _returnvalue _returnvalue_3))
      (bind _velocity (`MovementComponent.Velocity` _output_get))
      (set `self.Velocity` (+ (* _returnvalue_2 (`|EaseFunction` "Linear" (`KismetMathLibrary.Square` (`KismetMathLibrary.Dot_VectorVector` (`KismetMathLibrary.Normal` (- _returnvalue_3 _returnvalue)) (`KismetMathLibrary.Normal` _returnvalue_2))) 1.0 (`KismetMathLibrary.SelectFloat` (`KismetMathLibrary.MapRangeClamped` _returnvalue_4 0.0 4000.0 0.125 0.5) (`KismetMathLibrary.MapRangeClamped` _returnvalue_4 4000.0 16000.0 0.5 1.0) (<= _returnvalue_4 4000.0)))) _velocity)))
    (:`else`
      (set `self.Velocity` (+ _velocity _returnvalue_2))))
  (if (`self.Activated`)
    (set `self.Activated` false)
    (if (`self.Pull`)
      (for _array_element (`/Game/Game/Blueprint/BP_PlayerManager.Attachments` (`self.TargetManager`))
        (bind _asbp_grappling_hook (cast `/Game/Game/Blueprint/BP_GrapplingHook` (`ChildActorComponent.ChildActor` _array_element)))
        (set `/Game/Game/Blueprint/BP_GrapplingHook.Displacement` (0.0 0.0 0.0) _asbp_grappling_hook))
      (else
        (for _array_element_2 (`/Game/Game/Blueprint/BP_PlayerManager.Attachments` (`self.OwnManager`))
          (bind _asbp_grappling_hook_2 (cast `/Game/Game/Blueprint/BP_GrapplingHook` (`ChildActorComponent.ChildActor` _array_element_2)))
          (set `/Game/Game/Blueprint/BP_GrapplingHook.Displacement` (0.0 0.0 0.0) _asbp_grappling_hook_2))))
    (else
      (set `self.Activated` true)
      (set `self.Landed` false))))

(event `self.ReceiveTick`
  (params (DeltaSeconds :type "Float (single-precision)"))
  (bind _harpoon (`self.Harpoon`))
  (bind _targetmanager (`self.TargetManager`))
  (bind _ownmanager (`self.OwnManager`))
  (bind _harpoon_2 (`self.Harpoon`))
  (bind _returnvalue (`self.K2_GetActorLocation` _ownmanager))
  (bind _returnvalue_2 (`self.K2_GetActorLocation` (`self.TargetManager`)))
  (bind _visuals (`/Game/Game/Blueprint/BP_PlayerManager.Visuals` (`self.TargetManager`)))
  (bind _result (`|EaseFunction` "Linear" 0.01 _returnvalue_2 (`self.K2_GetActorLocation` (`self.OwnManager`))))
  (bind _result_2 (`|EaseFunction` "Linear" 0.01 _returnvalue (`SceneComponent.K2_GetComponentLocation` (`self.Sphere`))))
  (if (`self.Activated`)
    (if (`self.Landed`)
      (if (`self.Pull`)
        (`SceneComponent.K2_SetWorldLocationAndRotation` (`self.Harpoon`) (+ (`self.K2_GetActorLocation` _visuals) (`self.HarpoonRelativeLocation`)) (`KismetMathLibrary.ComposeRotators` (`self.K2_GetActorRotation` _visuals) (`self.HarpoonRelativeRotation`)) false false)
        (`self.K2_TeleportTo` _targetmanager _result (`self.K2_GetActorRotation` _targetmanager))
        (for _array_element (`/Game/Game/Blueprint/BP_PlayerManager.Attachments` (`self.TargetManager`))
          (bind _asbp_grappling_hook (cast `/Game/Game/Blueprint/BP_GrapplingHook` (`ChildActorComponent.ChildActor` _array_element)))
          (set `/Game/Game/Blueprint/BP_GrapplingHook.Displacement` (- _result _returnvalue_2) _asbp_grappling_hook))
        (else
          (`self.K2_TeleportTo` _ownmanager _result_2 (`self.K2_GetActorRotation` _ownmanager))
          (for _array_element_2 (`/Game/Game/Blueprint/BP_PlayerManager.Attachments` (`self.OwnManager`))
            (bind _asbp_grappling_hook_2 (cast `/Game/Game/Blueprint/BP_GrapplingHook` (`ChildActorComponent.ChildActor` _array_element_2)))
            (set `/Game/Game/Blueprint/BP_GrapplingHook.Displacement` (- _result_2 _returnvalue) _asbp_grappling_hook_2))))
      (else
        (set `self.Velocity` (- (`self.Velocity`) (0.0 0.0 10.0)))
        (`SceneComponent.K2_SetWorldLocation` _harpoon_2 (+ (* DeltaSeconds (`self.Velocity`)) (`SceneComponent.K2_GetComponentLocation` (`self.Harpoon`))) false false)
        (`KismetSystemLibrary.PrintString` "Hello")
        (`SceneComponent.K2_SetWorldRotation` _harpoon_2 (`KismetMathLibrary.MakeRotFromX` (- (`self.Velocity`) (`MovementComponent.Velocity` (`self.MovementRef`)))) false false)))
    (else
      (bind _movementref (`self.MovementRef`)
        (:`then`
          (`SceneComponent.K2_SetWorldLocation` _harpoon (+ (+ (`SceneComponent.K2_GetComponentLocation` (`self.Arrow`)) (* (`MovementComponent.Velocity` _movementref) DeltaSeconds)) (`self.Displacement`)) false false)
          (`SceneComponent.K2_SetWorldRotation` _harpoon (`SceneComponent.K2_GetComponentRotation` (`self.Arrow`)) false false))
        (:`else`)))))

(event `self.Sphere.OnComponentBeginOverlap`
  (params (OverlappedComponent :type "PrimitiveComponent Object Reference") (OtherActor :type "Actor Object Reference") (OtherComp :type "PrimitiveComponent Object Reference") (OtherBodyIndex :type Integer) (bFromSweep :type Boolean) (SweepResult :type "HitResult Structure (by ref)"))
  (bind _harpoon (`self.Harpoon`))
  (bind _harpoon_2 (`self.Harpoon`))
  (bind _harpoon_3 (`self.Harpoon`))
  (bind _returnvalue (`SceneComponent.K2_GetComponentLocation` (`self.Sphere`)))
  (bind _ownmanager (`self.OwnManager`)
    (:`then`
      (if (and (!= OtherActor (`/Game/Game/Blueprint/BP_PlayerManager.Visuals` _ownmanager)) (!= OtherActor _ownmanager))
        (if (not (`self.Landed`))
          (set `self.Landed` true)
          (bind _asbp_player_visuals (cast `/Game/Game/Blueprint/BP_PlayerVisuals` OtherActor)
            (:`then`
              (set `self.Pull` true)
              (set `self.TargetManager` (`/Game/Game/Blueprint/BP_PlayerVisuals.Manager` _asbp_player_visuals))
              (`KismetSystemLibrary.PrintString` "Hello")
              (set `self.HarpoonRelativeLocation` (- (`SceneComponent.K2_GetComponentLocation` _harpoon_3) (`self.K2_GetActorLocation` _asbp_player_visuals)))
              (set `self.HarpoonRelativeRotation` (`KismetMathLibrary.NormalizedDeltaRotator` (`self.K2_GetActorRotation` _asbp_player_visuals) (`SceneComponent.K2_GetComponentRotation` _harpoon_3))))
            (:`CastFailed`
              (bind _asbp_player_manager (cast `/Game/Game/Blueprint/BP_PlayerManager` OtherActor)
                (:`then`
                  (set `self.Pull` true)
                  (set `self.TargetManager` _asbp_player_manager)
                  (bind _visuals (`/Game/Game/Blueprint/BP_PlayerManager.Visuals` _asbp_player_manager))
                  (set `self.HarpoonRelativeLocation` (- (`SceneComponent.K2_GetComponentLocation` _harpoon_2) (`self.K2_GetActorLocation` _visuals)))
                  (set `self.HarpoonRelativeRotation` (`KismetMathLibrary.NormalizedDeltaRotator` (`self.K2_GetActorRotation` _visuals) (`SceneComponent.K2_GetComponentRotation` _harpoon_2))))
                (:`CastFailed`
                  (set `self.Pull` false)
                  (bind _outhit (`KismetSystemLibrary.SphereTraceSingle` _returnvalue _returnvalue (* (`KismetMathLibrary.MultiplyMultiply_FloatFloat` 1.5 (`KismetMathLibrary.Conv_IntToDouble` (`/Game/Game/Blueprint/BP_PlayerManager.Level` (`self.OwnManager`)))) 22.0) "TraceTypeQuery1"))
                  (`KismetSystemLibrary.Delay` 0.0)
                  (bind (_bblockinghit _binitialoverlap _time _distance _location _impactpoint _normal) (`GameplayStatics.BreakHitResult` _outhit))
                  (`SceneComponent.K2_SetWorldRotation` _harpoon (`KismetMathLibrary.MakeRotFromX` (`|EaseFunction` "Linear" 0.5 (`KismetMathLibrary.Normal` (`KismetMathLibrary.NegateVector` _normal)) (`KismetMathLibrary.Normal` (`SceneComponent.GetForwardVector` (`self.Harpoon`))))) false false)
                  (`SceneComponent.K2_SetWorldLocation` _harpoon (+ _location (* (0.0 0.0 50.0) (`KismetMathLibrary.MultiplyMultiply_FloatFloat` 1.5 (`KismetMathLibrary.Conv_IntToDouble` (`/Game/Game/Blueprint/BP_PlayerManager.Level` (`self.OwnManager`)))))) false false))))))))
    (:`else`)))

(fn `UserConstructionScript`
  (`parent.UserConstructionScript`))