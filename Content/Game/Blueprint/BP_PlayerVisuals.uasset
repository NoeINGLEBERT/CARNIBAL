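; BP_PlayerVisuals is the visual car actor paired with a player manager, in a game where higher-level cars eat lower-level ones.
; LevelUpdate sets scale, movement, meshes, headlight tint and claw per level.
; Tick drives skidmarks, fog parameters and the claw, which reacts to nearby cars and consumables.
; Overlapping a higher-level player destroys the manager, pulls the body into the killer, then awards scrap and respawns.
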(event `DeathServer`
  (`self.DeathClient`))

(event `DeathClient`
  (`self.K2_DestroyActor`))

(event `self.ReceiveTick`
  (params (DeltaSeconds :type "Float (single-precision)"))
  (bind (_returnvalue_x _returnvalue_y _returnvalue_z) (`KismetMathLibrary.BreakVector` (`self.K2_GetActorLocation`)))
  (bind (_returnvalue_x_2 _returnvalue_y_2 _returnvalue_z_2) (`KismetMathLibrary.BreakVector` (`self.GetActorForwardVector`)))
  (bind _killerref (`self.KillerRef`))
  (bind _killerref_2 (`self.KillerRef`))
  (bind _box (`self.Box`))
  (bind _box_2 (`/Game/Game/Blueprint/BP_PlayerVisuals.Box` (`/Game/Game/Blueprint/BP_PlayerManager.Visuals` (`self.KillerRef`))))
  (bind _returnvalue (+ (`SceneComponent.K2_GetComponentLocation` _box_2) (* (`SceneComponent.GetForwardVector` _box_2) 1.0)))
  (bind _returnvalue_2 (`KismetMathLibrary.FClamp` (/ (- (`GameplayStatics.GetTimeSeconds`) (`self.DeathTimeStamp`)) (/ (`self.KillerDistance`) (- (`KismetMathLibrary.Dot_VectorVector` (`self.GetActorForwardVector` _killerref) (`MovementComponent.Velocity` (`Character.CharacterMovement` _killerref))) (`self.DeathSpeed`))))))
  (if (!= (`self.KillerRef`) null)
    (`SceneComponent.K2_SetWorldLocation` (`self.Box`) (`|EaseFunction` "Linear" (- 1.0 _returnvalue_2) _returnvalue (+ _returnvalue (* (`SceneComponent.GetForwardVector` (`/Game/Game/Blueprint/BP_PlayerVisuals.TargetArrow` (`/Game/Game/Blueprint/BP_PlayerManager.Visuals` (`self.KillerRef`)))) (`self.KillerDistance`)))) false false)
    (`SceneComponent.K2_SetWorldRotation` _box (`|EaseFunction` "Linear" 0.2 (`SceneComponent.K2_GetComponentRotation` _box) (`SceneComponent.K2_GetComponentRotation` (`/Game/Game/Blueprint/BP_PlayerVisuals.Box` (`/Game/Game/Blueprint/BP_PlayerManager.Visuals` (`self.KillerRef`))))) false false)
    (if (== _returnvalue_2 1.0)
      (`/Engine/EditorBlueprintResources/StandardMacros.DoOnce` false
        (:`Completed`
          (`/Game/Game/Blueprint/BP_PlayerManager.ScrapUpdate` _killerref_2 (`KismetMathLibrary.FTrunc` (* (`KismetMathLibrary.Conv_IntToDouble` (`self.Scrap`)) 0.75)))
          (`FMODBlueprintStatics.PlayEventAttached` "/Game/FMOD/Events/SFX_Vehicle/Event_Vehicle_Crunch.Event_Vehicle_Crunch" (`/Game/Game/Blueprint/BP_PlayerManager.Box` _killerref_2) "None" (0.0 0.0 0.0) "KeepRelativeOffset")
          (bind _aspc_game_1 (cast `/Game/Game/Levels/Game1/PC_Game1` (`self.PlayerController`))
            (:`then`
              (`/Game/Game/Levels/Game1/PC_Game1.DeathHUDServer` _aspc_game_1))
            (:`CastFailed`
              _))
          (`KismetSystemLibrary.Delay` 4.0)
          (`self.DeathServer`)
          (bind _asgm_game_1 (cast `/Game/Game/Levels/Game1/GM_Game1` (`GameplayStatics.GetGameMode`)))
          (`/Game/Game/Levels/Game1/GM_Game1.Respawn` _asgm_game_1))))
    (else
      (`|ExecutionSequence`
        (:`then_0`
          (`/Engine/EditorBlueprintResources/StandardMacros.DoOnce` false
            (:`Completed`
              (bind _returnvalue_3 (`PrimitiveComponent.CreateDynamicMaterialInstance` (`self.Headlight`) 0 "/Game/Game/Materials/MI_Headlight.MI_Headlight" "None"))
              (set `self.HeadlightMaterial` _returnvalue_3)
              (`self.LevelUpdate` (`self.Level`)))))
        (:`then_1`
          (bind _manager (`self.Manager`)
            (:`then`
              (bind (_relativerotation_roll _relativerotation_pitch _relativerotation_yaw) (`KismetMathLibrary.BreakRotator` (`SceneComponent.RelativeRotation` (`/Game/Game/Blueprint/BP_PlayerManager.Box` _manager))))
              (`NiagaraComponent.SetVariableVec4` (`self.NS_Skidmark`) "Color" (`KismetMathLibrary.MakeVector4` 0.0 0.0 0.0 (`KismetMathLibrary.MapRangeClamped` (* (`KismetMathLibrary.Abs` (/ _relativerotation_yaw 10.0)) (/ (`KismetMathLibrary.MultiplyMultiply_FloatFloat` (* (`KismetMathLibrary.Dot_VectorVector` (`self.GetActorForwardVector`) (`MovementComponent.Velocity` (`Character.CharacterMovement` _manager))) 0.036) 2.0) 10000000.0)) 0.0 0.75 0.0 0.75)))
              (`NiagaraComponent.SetVariableVec4` (`self.NS_Skidmark1`) "Color" (`KismetMathLibrary.MakeVector4` 0.0 0.0 0.0 (`KismetMathLibrary.MapRangeClamped` (* (`KismetMathLibrary.Abs` (/ _relativerotation_yaw 10.0)) (/ (`KismetMathLibrary.MultiplyMultiply_FloatFloat` (* (`KismetMathLibrary.Dot_VectorVector` (`self.GetActorForwardVector`) (`MovementComponent.Velocity` (`Character.CharacterMovement` _manager))) 0.036) 2.0) 10000000.0)) 0.0 0.75 0.0 0.75)))
              (`NiagaraComponent.SetVariableVec4` (`self.NS_Skidmark2`) "Color" (`KismetMathLibrary.MakeVector4` 0.0 0.0 0.0 (`KismetMathLibrary.MapRangeClamped` (* (`KismetMathLibrary.Abs` (/ _relativerotation_yaw 10.0)) (/ (`KismetMathLibrary.MultiplyMultiply_FloatFloat` (* (`KismetMathLibrary.Dot_VectorVector` (`self.GetActorForwardVector`) (`MovementComponent.Velocity` (`Character.CharacterMovement` _manager))) 0.036) 2.0) 10000000.0)) 0.0 0.75 0.0 0.75)))
              (`NiagaraComponent.SetVariableVec4` (`self.NS_Skidmark3`) "Color" (`KismetMathLibrary.MakeVector4` 0.0 0.0 0.0 (`KismetMathLibrary.MapRangeClamped` (* (`KismetMathLibrary.Abs` (/ _relativerotation_yaw 10.0)) (/ (`KismetMathLibrary.MultiplyMultiply_FloatFloat` (* (`KismetMathLibrary.Dot_VectorVector` (`self.GetActorForwardVector`) (`MovementComponent.Velocity` (`Character.CharacterMovement` _manager))) 0.036) 2.0) 10000000.0)) 0.0 0.75 0.0 0.75)))
              (`self.SetActorScale3D` (`|EaseFunction` "Linear" 0.05 (`self.GetActorScale3D`) (`self.TargetScale`)))
              (`self.ClawManager`))
            (:`else`
              _))
          (if (== (`GameplayStatics.GetPlayerPawn` 0) (`self.Manager`))
            (`KismetMaterialLibrary.SetVectorParameterValue` "/Game/Game/Materials/MPC_Fog.MPC_Fog" "PlayerWorldLocation" (make `LinearColor` _returnvalue_x _returnvalue_y _returnvalue_z 1.0))
            (`KismetMaterialLibrary.SetVectorParameterValue` "/Game/Game/Materials/MPC_Fog.MPC_Fog" "PlayerForwardVector" (make `LinearColor` _returnvalue_x_2 _returnvalue_y_2 _returnvalue_z_2 1.0))
            (bind _returnvalue_4 (`KismetMaterialLibrary.GetScalarParameterValue` "/Game/Game/Materials/MPC_Fog.MPC_Fog" "HeadlightRange"))
            (`KismetMaterialLibrary.SetScalarParameterValue` "/Game/Game/Materials/MPC_Fog.MPC_Fog" "HeadlightRange" (`|EaseFunction` "Linear" 0.2 _returnvalue_4 (`self.HeadlightTargetRange`)))))))))

(event `self.Collider.OnComponentBeginOverlap`
  (params (OverlappedComponent :type "PrimitiveComponent Object Reference") (OtherActor :type "Actor Object Reference") (OtherComp :type "PrimitiveComponent Object Reference") (OtherBodyIndex :type Integer) (bFromSweep :type Boolean) (SweepResult :type "HitResult Structure (by ref)"))
  (bind _manager (`self.Manager`))
  (bind _returnvalue (`SceneComponent.GetForwardVector` (`/Game/Game/Blueprint/BP_PlayerVisuals.Box` (`/Game/Game/Blueprint/BP_PlayerManager.Visuals` (`self.KillerRef`)))))
  (if (!= OtherActor (`self.Manager`))
    (bind _asbp_player_manager (cast `/Game/Game/Blueprint/BP_PlayerManager` OtherActor))
    (if (> (`/Game/Game/Blueprint/BP_PlayerManager.Level` _asbp_player_manager) (`self.Level`))
      (`/Engine/EditorBlueprintResources/StandardMacros.DoOnce` false
        (:`Completed`
          (bind _output_get (set `self.KillerRef` _asbp_player_manager))
          (bind _box (`/Game/Game/Blueprint/BP_PlayerVisuals.Box` (`/Game/Game/Blueprint/BP_PlayerManager.Visuals` _output_get)))
          (bind _returnvalue_2 (- (`SceneComponent.K2_GetComponentLocation` (`self.Box`)) (+ (`SceneComponent.K2_GetComponentLocation` _box) (* (`SceneComponent.GetForwardVector` _box) 1.0))))
          (`SceneComponent.K2_SetWorldRotation` (`/Game/Game/Blueprint/BP_PlayerVisuals.TargetArrow` (`/Game/Game/Blueprint/BP_PlayerManager.Visuals` (`self.KillerRef`))) (`KismetMathLibrary.MakeRotFromX` _returnvalue_2) false false)
          (set `self.KillerDistance` (`KismetMathLibrary.VSize` _returnvalue_2))
          (set `self.DeathTimeStamp` (`GameplayStatics.GetTimeSeconds`))
          (bind _manager_2 (`self.Manager`)
            (:`then`
              (set `self.DeathSpeed` (`KismetMathLibrary.Dot_VectorVector` (`MovementComponent.Velocity` (`Character.CharacterMovement` _manager_2)) _returnvalue))
              (set `self.Scrap` (`/Game/Game/Blueprint/BP_PlayerManager.Scrap` _manager))
              (bind _asplayer_controller (cast `PlayerController` (`self.GetController` _manager))
                (:`then`
                  (set `self.PlayerController` _asplayer_controller))
                (:`CastFailed`
                  _))
              (`self.K2_DestroyActor` _manager))
            (:`else`
              (set `self.DeathSpeed` (`KismetMathLibrary.VSize` _returnvalue)))))))))

(event `self.ClawDetection.OnComponentBeginOverlap`
  (params (OverlappedComponent :type "PrimitiveComponent Object Reference") (OtherActor :type "Actor Object Reference") (OtherComp :type "PrimitiveComponent Object Reference") (OtherBodyIndex :type Integer) (bFromSweep :type Boolean) (SweepResult :type "HitResult Structure (by ref)"))
  (bind _visualsarray (`self.VisualsArray`))
  (bind _consumablearray (`self.ConsumableArray`))
  (if (!= OtherActor self)
    (bind _asbp_player_visuals (cast `/Game/Game/Blueprint/BP_PlayerVisuals` OtherActor)
      (:`then`
        (if (not (`KismetArrayLibrary.Array_Contains` _visualsarray _asbp_player_visuals))
          (`KismetArrayLibrary.Array_Add` _visualsarray _asbp_player_visuals)))
      (:`CastFailed`
        (bind _asbp_consumable (cast `/Game/Game/Blueprint/BP_Consumable` OtherActor))
        (if (not (`KismetArrayLibrary.Array_Contains` _consumablearray _asbp_consumable))
          (`KismetArrayLibrary.Array_Add` _consumablearray _asbp_consumable))))))

(event `self.ClawDetection.OnComponentEndOverlap`
  (params (OverlappedComponent :type "PrimitiveComponent Object Reference") (OtherActor :type "Actor Object Reference") (OtherComp :type "PrimitiveComponent Object Reference") (OtherBodyIndex :type Integer))
  (bind _visualsarray (`self.VisualsArray`))
  (bind _consumablearray (`self.ConsumableArray`))
  (if (!= OtherActor self)
    (bind _asbp_player_visuals (cast `/Game/Game/Blueprint/BP_PlayerVisuals` OtherActor)
      (:`then`
        (if (`KismetArrayLibrary.Array_Contains` _visualsarray _asbp_player_visuals)
          (`KismetArrayLibrary.Array_RemoveItem` _visualsarray _asbp_player_visuals)))
      (:`CastFailed`
        (bind _asbp_consumable (cast `/Game/Game/Blueprint/BP_Consumable` OtherActor))
        (if (`KismetArrayLibrary.Array_Contains` _consumablearray _asbp_consumable)
          (`KismetArrayLibrary.Array_RemoveItem` _consumablearray _asbp_consumable))))))

(fn `ClawManager`
  (bind _claw (`self.Claw`))
  (bind _visualsarray (`self.VisualsArray`))
  (bind _consumablearray (`self.ConsumableArray`))
  (bind _returnvalue (`KismetArrayLibrary.Array_IsEmpty` _consumablearray))
  (bind _returnvalue_2 (`SceneComponent.K2_GetComponentLocation` (`self.Arrow1`)))
  (bind _returnvalue_3 (`SceneComponent.K2_GetComponentLocation` (`self.Arrow1`)))
  (bind _returnvalue_4 (- (`self.K2_GetActorLocation` (`self.ClosestConsumable`)) (`SceneComponent.K2_GetComponentLocation` (`self.Arrow1`))))
  (bind _returnvalue_5 (- (`self.K2_GetActorLocation` (`self.ClosestConsumable`)) (`SceneComponent.K2_GetComponentLocation` (`self.Arrow1`))))
  (bind _returnvalue_6 (/ (`KismetMathLibrary.VSize` _returnvalue_4) (`KismetMathLibrary.Dot_VectorVector` (`KismetMathLibrary.Normal` _returnvalue_4) (`SceneComponent.GetForwardVector` (`self.Arrow1`)))))
  (bind _returnvalue_7 (/ (`KismetMathLibrary.VSize` _returnvalue_5) (`KismetMathLibrary.Dot_VectorVector` (`KismetMathLibrary.Normal` _returnvalue_5) (`SceneComponent.GetForwardVector` (`self.Arrow1`)))))
  (set `self.Distance` 10000.0)
  (if (`KismetArrayLibrary.Array_IsEmpty` _visualsarray)
    (if _returnvalue
      (`SkeletalMeshComponent.SetPosition` _claw (`|EaseFunction` "Linear" 0.1 (`SkeletalMeshComponent.GetPosition` _claw)) true)
      (else
        (set `self.ClosestConsumable` (`|GetArrayItem` _consumablearray) :!label _label)
        (for _array_element _consumablearray
          (if (< (`KismetMathLibrary.Vector_Distance` (`self.K2_GetActorLocation`) _returnvalue_3) (`KismetMathLibrary.Vector_Distance` _returnvalue_3 (`self.K2_GetActorLocation` (`self.ClosestConsumable`))))
            (set `self.ClosestConsumable` _array_element)
            (if (< _returnvalue_7 (`self.Distance`))
              (set `self.Distance` _returnvalue_7)
              (`SkeletalMeshComponent.SetPosition` (`self.Claw`) (`KismetMathLibrary.Square` (- 1.0 (/ (`self.Distance`) 5000.0))) true :!label _label_2))))))
    (else
      (set `self.ClosestTarget` (`|GetArrayItem` _visualsarray))
      (for _array_element_2 _visualsarray
        (if (< (`KismetMathLibrary.Vector_Distance` (`self.K2_GetActorLocation` _array_element_2) _returnvalue_2) (`KismetMathLibrary.Vector_Distance` _returnvalue_2 (`self.K2_GetActorLocation` (`self.ClosestTarget`))))
          (set `self.ClosestTarget` _array_element_2)
          (if (< _returnvalue_6 (`self.Distance`))
            (set `self.Distance` _returnvalue_6))))
      (if _returnvalue
        (goto _label_2)
        (else
          (goto _label))))))

(fn `Drift`
  (bind (_returnvalue_location _returnvalue_rotation) (`KismetMathLibrary.BreakTransform` (`SceneComponent.GetRelativeTransform` (`self.Box`))))
  (if (not (`self.IsDrifting`))
    (`SceneComponent.K2_SetRelativeRotation` (`self.Mesh`) (`|EaseFunction` "Linear" 0.05 _returnvalue_rotation) false false)
    (`SceneComponent.K2_SetRelativeRotation` (`self.Box`) (`|EaseFunction` "Linear" 0.05 _returnvalue_rotation) false false)))

(fn `Get Forward Speed`
  (returns (ReturnValue :type "Float (double-precision)"))
  (return (* (`KismetMathLibrary.Dot_VectorVector` (`self.GetActorForwardVector`) (`MovementComponent.Velocity` (`self.CharacterMovement`))) 0.036)))

(fn `LevelUpdate`
  (params (NewLevel :type Integer))
  (bind _charactermovement (`self.CharacterMovement`))
  (bind _output_get (set `self.Level` NewLevel))
  (switch `int` _output_get
    (:`0`
      (set `self.TargetScale` (0.8 0.8 0.8))
      (set `CharacterMovementComponent.MaxAcceleration` 1750.0 _charactermovement)
      (set `CharacterMovementComponent.MaxWalkSpeed` 6830.134554 _charactermovement)
      (set `self.TargetCameraBoomDistance` 768.0)
      (bind _headlightmaterial (`self.HeadlightMaterial`)
        (:`then`
          (`MaterialInstanceDynamic.SetScalarParameterValue` _headlightmaterial "Tint" 1.0)
          (`LightComponent.SetLightColor` (`self.RightSpotLight`) (struct :`R` 1.0 :`G` 1.0 :`A` 1.0) true)
          (`LightComponent.SetLightColor` (`self.LeftSpotLight`) (struct :`R` 1.0 :`G` 1.0 :`A` 1.0) true)
          (`StaticMeshComponent.SetStaticMesh` (`self.Car`) "/Game/Game/Anim/V1/SM_fleetline_Var_1_polySurface288.SM_fleetline_Var_1_polySurface288")
          (`StaticMeshComponent.SetStaticMesh` (`self.Headlight`) "/Game/Game/Anim/V1/SM_fleetline_Var_1_polySurface31.SM_fleetline_Var_1_polySurface31")
          (`StaticMeshComponent.SetStaticMesh` (`self.HeadlightOff`) "/Game/Game/Anim/V1/SM_fleetline_Var_1_polySurface31.SM_fleetline_Var_1_polySurface31")
          (`SkeletalMeshComponent.SetSkeletalMeshAsset` (`self.Claw`) "/Game/Game/Anim/SKM_CarAnimation.SKM_CarAnimation"))
        (:`else`)))
    (:`1`
      (set `self.TargetScale` (1.0 1.0 1.0))
      (set `CharacterMovementComponent.MaxAcceleration` 1500.0 _charactermovement)
      (set `CharacterMovementComponent.MaxWalkSpeed` 7513.148009 _charactermovement)
      (set `self.TargetCameraBoomDistance` 960.0)
      (bind _headlightmaterial_2 (`self.HeadlightMaterial`)
        (:`then`
          (`MaterialInstanceDynamic.SetScalarParameterValue` _headlightmaterial_2 "Tint" 0.75)
          (`LightComponent.SetLightColor` (`self.RightSpotLight`) (struct :`R` 1.0 :`G` 0.75 :`A` 1.0) true)
          (`LightComponent.SetLightColor` (`self.LeftSpotLight`) (struct :`R` 1.0 :`G` 0.75 :`A` 1.0) true)
          (`StaticMeshComponent.SetStaticMesh` (`self.Car`) "/Game/Game/Anim/V2/SM_fleetline_Var_2_pCylinder71.SM_fleetline_Var_2_pCylinder71")
          (`StaticMeshComponent.SetStaticMesh` (`self.Headlight`) "/Game/Game/Anim/V2/SM_fleetline_Var_2_polySurface31.SM_fleetline_Var_2_polySurface31")
          (`StaticMeshComponent.SetStaticMesh` (`self.HeadlightOff`) "/Game/Game/Anim/V2/SM_fleetline_Var_2_polySurface31.SM_fleetline_Var_2_polySurface31")
          (`SkeletalMeshComponent.SetSkeletalMeshAsset` (`self.Claw`) "/Game/Game/Anim/SKM_CarAnimation.SKM_CarAnimation"))
        (:`else`)))
    (:`2`
      (set `self.TargetScale` (1.25 1.25 1.25))
      (set `CharacterMovementComponent.MaxAcceleration` 1250.0 _charactermovement)
      (set `CharacterMovementComponent.MaxWalkSpeed` 8264.46281 _charactermovement)
      (set `self.TargetCameraBoomDistance` 1200.0)
      (bind _headlightmaterial_3 (`self.HeadlightMaterial`)
        (:`then`
          (`MaterialInstanceDynamic.SetScalarParameterValue` _headlightmaterial_3 "Tint" 0.5)
          (`LightComponent.SetLightColor` (`self.RightSpotLight`) (struct :`R` 1.0 :`G` 0.5 :`A` 1.0) true)
          (`LightComponent.SetLightColor` (`self.LeftSpotLight`) (struct :`R` 1.0 :`G` 0.5 :`A` 1.0) true)
          (`StaticMeshComponent.SetStaticMesh` (`self.Car`) "/Game/Game/Anim/V3/SM_fleetline_Var_3_polySurface545.SM_fleetline_Var_3_polySurface545")
          (`StaticMeshComponent.SetStaticMesh` (`self.Headlight`) "/Game/Game/Anim/V3/SM_fleetline_Var_3_polySurface31.SM_fleetline_Var_3_polySurface31")
          (`StaticMeshComponent.SetStaticMesh` (`self.HeadlightOff`) "/Game/Game/Anim/V3/SM_fleetline_Var_3_polySurface31.SM_fleetline_Var_3_polySurface31")
          (`SkeletalMeshComponent.SetSkeletalMeshAsset` (`self.Claw`) "/Game/Game/Anim/SKM_CarAnimation.SKM_CarAnimation"))
        (:`else`)))
    (:`3`
      (set `self.TargetScale` (1.5625 1.5625 1.5625))
      (set `CharacterMovementComponent.MaxAcceleration` 1000.0 _charactermovement)
      (set `CharacterMovementComponent.MaxWalkSpeed` 9090.909091 _charactermovement)
      (set `self.TargetCameraBoomDistance` 1500.0)
      (bind _headlightmaterial_4 (`self.HeadlightMaterial`)
        (:`then`
          (`MaterialInstanceDynamic.SetScalarParameterValue` _headlightmaterial_4 "Tint" 0.25)
          (`LightComponent.SetLightColor` (`self.RightSpotLight`) (struct :`R` 1.0 :`G` 0.25 :`A` 1.0) true)
          (`LightComponent.SetLightColor` (`self.LeftSpotLight`) (struct :`R` 1.0 :`G` 0.25 :`A` 1.0) true)
          (`StaticMeshComponent.SetStaticMesh` (`self.Car`) "/Game/Game/Anim/V4/SM_fleetline_Var_4_polySurface547.SM_fleetline_Var_4_polySurface547")
          (`StaticMeshComponent.SetStaticMesh` (`self.Headlight`) "/Game/Game/Anim/V4/SM_fleetline_Var_4_polySurface236.SM_fleetline_Var_4_polySurface236")
          (`StaticMeshComponent.SetStaticMesh` (`self.HeadlightOff`) "/Game/Game/Anim/V4/SM_fleetline_Var_4_polySurface236.SM_fleetline_Var_4_polySurface236")
          (`SkeletalMeshComponent.SetSkeletalMeshAsset` (`self.Claw`) "/Game/Game/Anim/AnimV5/SKM_BoucheAnimation_var5_fleetline.SKM_BoucheAnimation_var5_fleetline"))
        (:`else`)))
    (:`4`
      (set `self.TargetScale` (1.953125 1.953125 1.953125))
      (set `CharacterMovementComponent.MaxAcceleration` 750.0 _charactermovement)
      (set `CharacterMovementComponent.MaxWalkSpeed` 10000.0 _charactermovement)
      (set `self.TargetCameraBoomDistance` 1875.0)
      (bind _headlightmaterial_5 (`self.HeadlightMaterial`)
        (:`then`
          (`MaterialInstanceDynamic.SetScalarParameterValue` _headlightmaterial_5 "Tint" 0.0)
          (`LightComponent.SetLightColor` (`self.RightSpotLight`) (struct :`R` 1.0 :`A` 1.0) true)
          (`LightComponent.SetLightColor` (`self.LeftSpotLight`) (struct :`R` 1.0 :`A` 1.0) true)
          (`StaticMeshComponent.SetStaticMesh` (`self.Car`) "/Game/Game/Anim/V5/SM_fleetline_Var_5_polySurface548.SM_fleetline_Var_5_polySurface548")
          (`StaticMeshComponent.SetStaticMesh` (`self.Headlight`) "/Game/Game/Anim/V5/SM_fleetline_Var_5_polySurface263.SM_fleetline_Var_5_polySurface263")
          (`StaticMeshComponent.SetStaticMesh` (`self.HeadlightOff`) "/Game/Game/Anim/V5/SM_fleetline_Var_5_polySurface263.SM_fleetline_Var_5_polySurface263")
          (`SkeletalMeshComponent.SetSkeletalMeshAsset` (`self.Claw`) "/Game/Game/Anim/AnimV5/SKM_BoucheAnimation_var5_fleetline.SKM_BoucheAnimation_var5_fleetline"))
        (:`else`)))))

(fn `UserConstructionScript`
  (`self.LevelUpdate` (`self.Level`))
  (`self.SetActorScale3D` (`self.TargetScale`)))

(fn `VisualTeleport`
  (bind _frw (`self.FRW`))
  (bind _flw (`self.FLW`))
  (bind _rrw (`self.RRW`))
  (bind _rlw (`self.RLW`))
  (`self.K2_TeleportTo` (/ (+ (`self.FRW`) (`self.RRW`)) 2.0) (`KismetMathLibrary.MakeRotFromXY` (+ (- _frw _rrw) (- _flw _rlw)) (+ (- _frw _flw) (- _rrw _rlw)))))